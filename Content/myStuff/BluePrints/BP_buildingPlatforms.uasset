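; Building platform Blueprint that grows or shrinks along Z by scaling its PointB component.
; StartEvent adds a signed MoveValue to the Z scale each tick, re-calling itself after a one-tick delay until it reaches MaxZScale or the 0.5 minimum.
; The construction script shows PointB at full extension, and BeginPlay resets it to the minimum.
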(event `/Game/myStuff/BluePrints/BP_Interfaces/BPI_Startable.StartEvent`
  (params (`Move Value` :type "Float (double-precision)"))
  (bind _pointb (`self.pointB`))
  (bind (_returnvalue_x _returnvalue_y _returnvalue_z) (`KismetMathLibrary.BreakVector` (`SceneComponent.K2_GetComponentScale` _pointb)))
  (bind (_returnvalue_x_2 _returnvalue_y_2 _returnvalue_z_2) (`KismetMathLibrary.BreakVector` (`SceneComponent.K2_GetComponentScale` (`self.pointB`))))
  ; Scaling/Unscaling the platform
  (`KismetSystemLibrary.DelayUntilNextTick`)
  (`SceneComponent.SetWorldScale3D` _pointb (`KismetMathLibrary.MakeVector` _returnvalue_x _returnvalue_y (`KismetMathLibrary.FClamp` (+ _returnvalue_z `Move Value`) 0.5 (`self.maxZScale`))))
  (if (not (== _returnvalue_z_2 (select `bool` (> `Move Value` 0.0) :`false` 0.5 :`true` (`self.maxZScale`))))
    (`/Game/myStuff/BluePrints/BP_Interfaces/BPI_Startable.StartEvent` `Move Value`)))

(event `self.ReceiveBeginPlay`
  (bind _pointb (`self.pointB`))
  (bind (_returnvalue_x _returnvalue_y) (`KismetMathLibrary.BreakVector` (`SceneComponent.K2_GetComponentScale` _pointb)))
  ; setting the scaling Back to normal
  (`SceneComponent.SetWorldScale3D` _pointb (`KismetMathLibrary.MakeVector` _returnvalue_x _returnvalue_y 0.5)))

(fn `UserConstructionScript`
  (bind _pointb (`self.pointB`))
  (bind (_returnvalue_x _returnvalue_y) (`KismetMathLibrary.BreakVector` (`SceneComponent.K2_GetComponentScale` _pointb)))
  (`SceneComponent.SetWorldScale3D` _pointb (`KismetMathLibrary.MakeVector` _returnvalue_x _returnvalue_y (`self.maxZScale`))))
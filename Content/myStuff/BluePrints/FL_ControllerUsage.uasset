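; FL_ControllerUsage is a function library with helpers for controller-driven menu highlighting and player overlap checks.
; ControllerWidgetUsage loops over buttons, copying the Hovered style into Normal for whichever has keyboard focus.
; The other buttons take their Normal style back from a parallel ButtonStyle array.
; CastToPlayer casts an actor to BP_ThirdPersonCharacter and returns whether the given component is its capsule.
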(fn `CastToPlayer`
  (params (`Other Actor` :type "Object Object Reference") (`Other Component` :type "Object Object Reference"))
  (returns (cast :type Boolean))
  (bind _asbp_third_person_character (cast `/Game/ThirdPerson/Blueprints/BP_ThirdPersonCharacter` `Other Actor`))
  (return (== (`Character.CapsuleComponent` _asbp_third_person_character) `Other Component`)))

(fn `ControllerWidgetUsage`
  (params (Buttons :type "Array of Button Object Reference") (ButtonStyle :type "Array of ButtonStyle Structure"))
  (for (_array_element _array_index) Buttons
    (if (`Widget.HasKeyboardFocus` _array_element)
      (bind _widgetstyle (`Button.WidgetStyle` _array_element))
      (setmembers `ButtonStyle` :`StructRef` _widgetstyle :`Normal` (`.Hovered` (break `ButtonStyle` _widgetstyle)))
      (else
        (setmembers `ButtonStyle` :`StructRef` _widgetstyle :`Normal` (`.Normal` (break `ButtonStyle` (`|GetArrayItem` ButtonStyle _array_index))))))))
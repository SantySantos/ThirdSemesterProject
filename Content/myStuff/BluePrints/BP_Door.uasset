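; BP_Door is a door that moves by shrinking the world Z scale of its PointB component.
; Construction and BeginPlay both set that scale to MaxZScale.
; StartEvent re-calls itself after a one-tick delay, subtracting MoveValue each step while the clamped result stays above MinZScale.
; The step is per tick rather than time-scaled, and the file contains no reverse movement.
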(event `/Game/myStuff/BluePrints/BP_Interfaces/BPI_Startable.StartEvent`
  (params (`Move Value` :type "Float (double-precision)"))
  (bind _pointb (`self.PointB`))
  (bind (_returnvalue_x _returnvalue_y _returnvalue_z) (`KismetMathLibrary.BreakVector` (`SceneComponent.K2_GetComponentScale` _pointb)))
  (bind _returnvalue (`KismetMathLibrary.FClamp` (- _returnvalue_z `Move Value`) (`self.MinZScale`) (`self.MaxZScale`)))
  ; Moving the door
  (`KismetSystemLibrary.DelayUntilNextTick`)
  (if (< (`self.MinZScale`) _returnvalue)
    (`SceneComponent.SetWorldScale3D` _pointb (`KismetMathLibrary.MakeVector` _returnvalue_x _returnvalue_y _returnvalue))
    (`/Game/myStuff/BluePrints/BP_Interfaces/BPI_Startable.StartEvent` `Move Value`)))

(event `self.ReceiveBeginPlay`
  (bind _pointb (`self.PointB`))
  (bind (_returnvalue_x _returnvalue_y) (`KismetMathLibrary.BreakVector` (`SceneComponent.K2_GetComponentScale` _pointb)))
  ; Setting the door Z Scale
  (`SceneComponent.SetWorldScale3D` _pointb (`KismetMathLibrary.MakeVector` _returnvalue_x _returnvalue_y (`self.MaxZScale`))))

(fn `UserConstructionScript`
  (bind _pointb (`self.PointB`))
  (bind (_returnvalue_x _returnvalue_y) (`KismetMathLibrary.BreakVector` (`SceneComponent.K2_GetComponentScale` _pointb)))
  (`SceneComponent.SetWorldScale3D` _pointb (`KismetMathLibrary.MakeVector` _returnvalue_x _returnvalue_y (`self.MaxZScale`))))
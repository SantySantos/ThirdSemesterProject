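; BP_LightSwitch is an interactable switch that toggles a set of lights when the player presses F nearby.
; A sphere collision enables input for player controller 0 when the third-person character's capsule enters, and disables it on exit.
; Pressing F loops through the LightsToSwitch array and inverts each light component's visibility, with debug messages printed along the way.
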(event `Key|F` :consume false
  (params (Key :type "Key Structure"))
  ; Turning on/off the lights
  (:`Pressed`
    (`KismetSystemLibrary.PrintString` "F was pressed")
    (for _array_element (`self.lightsToSwitch`)
      (bind _lightcomponent (`Light.LightComponent` _array_element))
      (`SceneComponent.SetVisibility` _lightcomponent (not (`SceneComponent.bVisible` _lightcomponent)) false))))

(event `self.SphereCollition.OnComponentBeginOverlap`
  (params (OverlappedComponent :type "PrimitiveComponent Object Reference") (OtherActor :type "Actor Object Reference") (OtherComp :type "PrimitiveComponent Object Reference") (OtherBodyIndex :type Integer) (bFromSweep :type Boolean) (SweepResult :type "HitResult Structure (by ref)"))
  ; Check if the character is close to the button
  (bind _asbp_third_person_character (cast `/Game/ThirdPerson/Blueprints/BP_ThirdPersonCharacter` OtherActor))
  (if (== (`Character.CapsuleComponent` _asbp_third_person_character) OtherComp)
    (`self.EnableInput` (`GameplayStatics.GetPlayerController` 0))
    (`KismetSystemLibrary.PrintString` "You can turn on the lights")))

(event `self.SphereCollition.OnComponentEndOverlap`
  (params (OverlappedComponent :type "PrimitiveComponent Object Reference") (OtherActor :type "Actor Object Reference") (OtherComp :type "PrimitiveComponent Object Reference") (OtherBodyIndex :type Integer))
  ; dont allow the player turn on/off lights if he left the button zone
  (bind _asbp_third_person_character (cast `/Game/ThirdPerson/Blueprints/BP_ThirdPersonCharacter` OtherActor))
  (if (== (`Character.CapsuleComponent` _asbp_third_person_character) OtherComp)
    (`self.DisableInput` (`GameplayStatics.GetPlayerController` 0))
    (`KismetSystemLibrary.PrintString` "Cant turn on Lights")))

(fn `UserConstructionScript`)
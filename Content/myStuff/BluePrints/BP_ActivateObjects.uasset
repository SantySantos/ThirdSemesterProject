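; BP_ActivateObjects is a trigger that drives a list of Activatable actors when a BP_FiringCube's collision component enters its box.
; On overlap it compares the cube's material to its own, plays audio with an isCorrect parameter, and on a match sends StartEventMessage with a positive value through BPI_Startable.
; On exit it sends the negative value to reverse them, without rechecking the material.
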(event `self.Box.OnComponentBeginOverlap`
  (params (OverlappedComponent :type "PrimitiveComponent Object Reference") (OtherActor :type "Actor Object Reference") (OtherComp :type "PrimitiveComponent Object Reference") (OtherBodyIndex :type Integer) (bFromSweep :type Boolean) (SweepResult :type "HitResult Structure (by ref)"))
  (bind _audio (`self.Audio`))
  ; Collides with the right object, execute
  (bind _asbp_firing_cube (cast `/Game/myStuff/BluePrints/BP_FiringCube` OtherActor))
  (if (== (`/Game/myStuff/BluePrints/BP_FiringCube.Collition` _asbp_firing_cube) OtherComp)
    (`KismetSystemLibrary.PrintString` "GoingUp")
    (`KismetSystemLibrary.PrintString` "Cube is here")
    (bind _returnvalue (== (`PrimitiveComponent.GetMaterial` (`self.Cube`) 0) (`PrimitiveComponent.GetMaterial` (`/Game/myStuff/BluePrints/BP_FiringCube.Cube` _asbp_firing_cube) 0)))
    (if _returnvalue
      (`AudioParameterControllerInterface.SetBoolParameter` _audio "isCorrect" _returnvalue)
      (`AudioComponent.Play` _audio 0.0)
      (for _array_element (`self.Activatable`)
        (if (`KismetSystemLibrary.DoesImplementInterface` _array_element "/Game/myStuff/BluePrints/BP_Interfaces/BPI_Startable.BPI_Startable_C")
          (message `/Game/myStuff/BluePrints/BP_Interfaces/BPI_Startable.StartEvent` _array_element 0.1)))
      (else
        (`AudioParameterControllerInterface.SetBoolParameter` _audio "isCorrect" _returnvalue)
        (`AudioComponent.Play` _audio 0.0)))))

(event `self.Box.OnComponentEndOverlap`
  (params (OverlappedComponent :type "PrimitiveComponent Object Reference") (OtherActor :type "Actor Object Reference") (OtherComp :type "PrimitiveComponent Object Reference") (OtherBodyIndex :type Integer))
  ; Checking Collition leaves
  (bind _asbp_firing_cube (cast `/Game/myStuff/BluePrints/BP_FiringCube` OtherActor))
  (if (== (`/Game/myStuff/BluePrints/BP_FiringCube.Collition` _asbp_firing_cube) OtherComp)
    (for _array_element (`self.Activatable`)
      (if (`KismetSystemLibrary.DoesImplementInterface` _array_element "/Game/myStuff/BluePrints/BP_Interfaces/BPI_Startable.BPI_Startable_C")
        (message `/Game/myStuff/BluePrints/BP_Interfaces/BPI_Startable.StartEvent` _array_element -0.1)))))

(fn `UserConstructionScript`)